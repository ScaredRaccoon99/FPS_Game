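; BP_Security_Camera is a stealth-game security camera that swings between two rotations and catches the first-person player.
; A looping MoveCamera event uses a FlipFlop to alternate target rotations for MoveComponentTo, pausing with a Delay.
; Each Tick, a debug-drawn forward line trace from SMLineTrace looks for Pawns; hitting the player sets Caught and disables input.
; The delayed StealthMap restart is left unconnected.
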(event `self.ReceiveBeginPlay`
  (`self.MoveCamera`)
  (bind _asbp_first_person_character (cast `/Game/StarterContent/FirstPersonArms/FirstPerson/Blueprints/BP_FirstPersonCharacter` (`GameplayStatics.GetPlayerCharacter` 0)))
  (set `self. BP First Person Character` _asbp_first_person_character))

(event `MoveCamera`
  (bind (_currentrotation_x _currentrotation_y _currentrotation_z) (`KismetMathLibrary.BreakVector` (`self.CurrentRotation`)))
  ; Move Camera
  (`/Engine/EditorBlueprintResources/StandardMacros.FlipFlop`
    (:`A`
      (set `self.CurrentRotation` (`self.EndRotation`)))
    (:`B`
      (set `self.CurrentRotation` (`self.StartRotation`))))
  (`KismetSystemLibrary.MoveComponentTo` (`self.SM_Camera`) (0.0 0.0 0.0) (`KismetMathLibrary.MakeRotator` _currentrotation_x _currentrotation_y _currentrotation_z) false false (`self.Speed`))
  (`KismetSystemLibrary.Delay` (`self.Delay`))
  (`self.MoveCamera`))

(event `self.ReceiveTick`
  (params (DeltaSeconds :type "Float (single-precision)"))
  (`self.Detect`))

(event `Detect`
  (bind _sm_linetrace (`self.SM_LineTrace`))
  (bind __bp_first_person_character (`self. BP First Person Character`))
  (bind _returnvalue (`SceneComponent.K2_GetComponentLocation` _sm_linetrace))
  ; Camera Detecion
  (bind _outhit (`KismetSystemLibrary.LineTraceSingleForObjects` :`Start` _returnvalue :`End` (+ _returnvalue (* (`KismetMathLibrary.GetForwardVector` (`SceneComponent.K2_GetComponentRotation` _sm_linetrace)) (`self.DetectDistance`))) :`ObjectTypes` (`|MakeArray` "ObjectTypeQuery3" :!type "EObjectTypeQuery Enum") :`DrawDebugType` "ForOneFrame"))
  (if (== (`.HitActor` (`GameplayStatics.BreakHitResult` _outhit)) __bp_first_person_character)
    (set `/Game/StarterContent/FirstPersonArms/FirstPerson/Blueprints/BP_FirstPersonCharacter.Caught` true __bp_first_person_character)
    ; Disable Input & Level Restart
    (`self.DisableInput` (`self. BP First Person Character`) (`GameplayStatics.GetPlayerController` 0))))

(fn `UserConstructionScript`)